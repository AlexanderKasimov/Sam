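; Paper2D side-view player character that runs along the X axis and jumps from player input.
; Each Tick mirrors the flipbook by the sign of X velocity, keeping the last facing when stopped, then updates the animation.
; GetAnimationState derives Idle, Walking, Jumping or Falling purely from velocity, without a movement-mode or ground check.
; UpdateAnimation maps that state to Sam's looping flipbooks, requesting play-from-start for jump and fall.
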(event `self.ReceiveTick`
  (params (DeltaSeconds :type "Float (single-precision)"))
  (bind _returnvalue (`KismetMathLibrary.SignOfFloat` (.x (`self.GetVelocity`))))
  (`|ExecutionSequence`
    (:`then_0`
      (if (not (`KismetMathLibrary.NearlyEqual_FloatFloat` _returnvalue))
        (`SceneComponent.SetWorldScale3D` (`self.PaperFlipbook`) (`KismetMathLibrary.MakeVector` _returnvalue 1.0 1.0))))
    (:`then_1`
      (`self.UpdateAnimation`))))

(event `InputAxis|MoveRight`
  (params (AxisValue :type "Float (single-precision)"))
  (`PawnMovementComponent.AddInputVector` (`self.CharacterMovement`) (`KismetMathLibrary.Normal` (`KismetMathLibrary.MakeVector` AxisValue)) false))

(event `InputAction|Jump`
  (params (Key :type "Key Structure"))
  (:`Pressed`
    (`self.Jump`)))

(fn `GetAnimationState`
  (returns (AnimState :type "/Game/BP/Enum/AnimationState_Enum Enum"))
  (if (> (.z (`self.GetVelocity`)) 1.0)
    (return "NewEnumerator2")
    (elif (< (.z (`self.GetVelocity`)) -1.0)
      (return "NewEnumerator3")
      (elif (> (`KismetMathLibrary.VSize` (`self.GetVelocity`)) 1.0)
        (return "NewEnumerator1")
        (else
          (return "NewEnumerator0"))))))

(fn `UpdateAnimation`
  (switch `/Game/BP/Enum/AnimationState_Enum` (`self.GetAnimationState`)
    (:`NewEnumerator0`
      (`/Game/BP/FL/FL_FlipbookComponent.SetFlipbook` "/Game/Sprites/Characters/Sam/Sam_Idle_FB.Sam_Idle_FB" (`self.PaperFlipbook`) true))
    (:`NewEnumerator1`
      (`/Game/BP/FL/FL_FlipbookComponent.SetFlipbook` "/Game/Sprites/Characters/Sam/Sam_Run_FB.Sam_Run_FB" (`self.PaperFlipbook`) true))
    (:`NewEnumerator2`
      (`/Game/BP/FL/FL_FlipbookComponent.SetFlipbook` "/Game/Sprites/Characters/Sam/Sam_Jump_FB.Sam_Jump_FB" (`self.PaperFlipbook`) true true))
    (:`NewEnumerator3`
      (`/Game/BP/FL/FL_FlipbookComponent.SetFlipbook` "/Game/Sprites/Characters/Sam/Sam_Fall_FB.Sam_Fall_FB" (`self.PaperFlipbook`) true true))))

(fn `UserConstructionScript`)