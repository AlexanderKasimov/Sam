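; Orthographic side-view camera actor that follows the player character in the XZ plane at a fixed Y depth.
; Tick starts following once the player is WindowSizeX away, then lerps by InterpSpeed and delta time until nearly centred.
; ChangeOrthoWidth plays a width timeline and enables cinematic mode, which lerps toward TargetActor instead and is never cleared here.
; Disconnected nodes hold an unused velocity-based follow variant.
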(event `ChangeOrthoWidth`
  (`|ExecutionSequence`
    (:`then_0`
      (bind (_direction _width) (`Timeline|Timeline_0`)
        (:`Update`
          (`CameraComponent.SetOrthoWidth` (`self.Camera`) _width))))
    (:`then_1`
      (set `self.InterpSpeed` 1.0)
      (set `self.isCinematic` true))))

(event `self.ReceiveBeginPlay`
  (`CameraComponent.SetOrthoWidth` (`self.Camera`) (`self.OrthoWidth`)))

(event `self.ReceiveTick`
  (params (DeltaSeconds :type "Float (single-precision)"))
  (if (not (`self.isCinematic`))
    (`|ExecutionSequence`
      (:`then_0`
        (if (>= (`KismetMathLibrary.VSize` (- (`KismetMathLibrary.MakeVector` (.x (`self.K2_GetActorLocation`)) 0.0 (.z (`self.K2_GetActorLocation`))) (`KismetMathLibrary.MakeVector` (.x (`self.K2_GetActorLocation` (`GameplayStatics.GetPlayerCharacter` 0))) 0.0 (.z (`self.K2_GetActorLocation` (`GameplayStatics.GetPlayerCharacter` 0)))))) (`self.WindowSizeX`))
          (set `self.isFollow` true)))
      (:`then_1`
        (if (`self.isFollow`)
          (if (`KismetMathLibrary.NearlyEqual_FloatFloat` (`KismetMathLibrary.VSize` (- (`KismetMathLibrary.MakeVector` (.x (`self.K2_GetActorLocation`)) 0.0 (.z (`self.K2_GetActorLocation`))) (`KismetMathLibrary.MakeVector` (.x (`self.K2_GetActorLocation` (`GameplayStatics.GetPlayerCharacter` 0))) 0.0 (.z (`self.K2_GetActorLocation` (`GameplayStatics.GetPlayerCharacter` 0)))))))
            (set `self.isFollow` false)
            (else
              (`self.K2_SetActorLocation` (`KismetMathLibrary.VLerp` (`self.K2_GetActorLocation`) (`KismetMathLibrary.MakeVector` (.x (`self.K2_GetActorLocation` (`GameplayStatics.GetPlayerCharacter` 0))) 200.0 (.z (`self.K2_GetActorLocation` (`GameplayStatics.GetPlayerCharacter` 0)))) (* (`self.InterpSpeed`) (`GameplayStatics.GetWorldDeltaSeconds`))))))))
      (:`then_2`
        (`/Game/BP/FL/FL_Debug.DebugBox` false (`self.K2_GetActorLocation`) (4.0 0.0 4.0) (struct :`R` 0.102331 :`G` 1.0 :`A` 1.0))))
    (else
      (`self.K2_SetActorLocation` (`KismetMathLibrary.VLerp` (`self.K2_GetActorLocation`) (`KismetMathLibrary.MakeVector` (.x (`self.K2_GetActorLocation` (`self.TargetActor`))) 200.0 (.z (`self.K2_GetActorLocation` (`self.TargetActor`)))) (* (`self.InterpSpeed`) (`GameplayStatics.GetWorldDeltaSeconds`)))))))

(fn `UserConstructionScript`
  (`CameraComponent.SetOrthoWidth` (`self.Camera`) (`self.OrthoWidth`)))