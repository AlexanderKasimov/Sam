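; BP_Pawn_Player is a player pawn that moves along the world X axis from the MoveRight input.
; Each Tick it normalizes that input into a direction, scales it by WalkSpeed and delta time, and offsets the actor location with a swept move.
; Normalizing discards analog magnitude, and the other events and construction script add no logic of their own.
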(event `self.ReceiveTick`
  (params (DeltaSeconds :type "Float (single-precision)"))
  (`self.K2_SetActorLocation` (+ (`self.K2_GetActorLocation`) (* (`KismetMathLibrary.Normal` (`KismetMathLibrary.MakeVector` (`self.GetInputAxisValue`))) (* (`self.WalkSpeed`) (`GameplayStatics.GetWorldDeltaSeconds`)))) true))

(fn `UserConstructionScript`
  (`parent.UserConstructionScript`))