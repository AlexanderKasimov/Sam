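; Parallax sprite actor that shifts with the BP_Camera to create depth in a 2D scene on the XZ plane.
; The construction script caches the first BP_Camera found, applies the sprite, X/Z offsets and scale, and stores the root's default location.
; Each tick, MoveActor sets the root to that location plus the camera's X and Z distance from it, multiplied by ParallaxCoef.
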(event `self.ReceiveBeginPlay`)

(event `self.ReceiveTick`
  (params (DeltaSeconds :type "Float (single-precision)"))
  (`self.MoveActor` (`self.ParallaxCoef`) (`self.DefaultSceneRoot`) (`self.DefaultLocation`)))

(fn `MoveActor`
  (params (ParallaxCoef :type "Float (double-precision)") (Actor :type "SceneComponent Object Reference") (ActorDefaultLocation :type "Vector Structure"))
  (locals (ParallaxCoefLocal :type "Float (double-precision)") (DefaultLocationLocal :type "Vector Structure") (SpriteComponent :type "PaperSpriteComponent Object Reference") (SceneComponent :type "SceneComponent Object Reference"))
  (set `local.SceneComponent` Actor)
  (set `local.ParallaxCoefLocal` ParallaxCoef)
  (set `local.DefaultLocationLocal` ActorDefaultLocation)
  (`/Engine/EditorBlueprintResources/StandardMacros.IsValid` (`local.SceneComponent`)
    (:`Is Valid`
      (`SceneComponent.K2_SetWorldLocation` (`local.SceneComponent`) (+ (`local.DefaultLocationLocal`) (`KismetMathLibrary.MakeVector` (.x (* (- (`self.K2_GetActorLocation` (`self.Camera`)) (`local.DefaultLocationLocal`)) (`local.ParallaxCoefLocal`))) 0.0 (.z (* (- (`self.K2_GetActorLocation` (`self.Camera`)) (`local.DefaultLocationLocal`)) (`local.ParallaxCoefLocal`))))) false false))))

(fn `UserConstructionScript`
  (`|ExecutionSequence`
    (:`then_0`
      (bind _outactors (`GameplayStatics.GetAllActorsOfClass` "/Game/BP/BP_Camera.BP_Camera_C"))
      (set `self.Camera` (`|GetArrayItem` _outactors)))
    (:`then_1`
      (`PaperSpriteComponent.SetSprite` (`self.PaperSprite`) (`self.Sprite`))
      (`SceneComponent.K2_SetWorldLocation` (`self.PaperSprite`) (`KismetMathLibrary.MakeVector` (+ (`self.XOffset`) (.x (`SceneComponent.K2_GetComponentLocation` (`self.PaperSprite`)))) (.y (`SceneComponent.K2_GetComponentLocation` (`self.PaperSprite`))) (+ (.z (`SceneComponent.K2_GetComponentLocation` (`self.PaperSprite`))) (`self.ZOffset`))) false false)
      (set `self.DefaultLocation` (`SceneComponent.K2_GetComponentLocation` (`self.DefaultSceneRoot`)))
      (`SceneComponent.SetWorldScale3D` (`self.DefaultSceneRoot`) (`KismetMathLibrary.Conv_DoubleToVector` (`self.Scale`))))))