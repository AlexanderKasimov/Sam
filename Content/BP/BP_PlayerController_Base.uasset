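; Base player controller that runs dialog sessions and provides debug hotkeys.
; StartDialog creates and shows a UI_Dialog widget and disables pawn input, while the Use action advances frames during dialog.
; EndDialog restores pawn input and calls DialogEnded.
; Function keys run console commands for performance stats and flip-flop toggles of view mode, screen percentage and resolution.
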(event `self.ReceiveBeginPlay`)

(event `self.ReceiveTick`
  (params (DeltaSeconds :type "Float (single-precision)")))

(event `InputAction|Use` :consume false
  (params (Key :type "Key Structure"))
  (:`Pressed`
    (if (`self.inDialog`)
      (`/Game/UI/UI_Dialog.NextFrame` (`self.DialogWidgetRef`)))))

(event `Key|F1`
  (params (Key :type "Key Structure"))
  (:`Pressed`
    (`KismetSystemLibrary.ExecuteConsoleCommand` "stat fps" null)))

(event `Key|F2`
  (params (Key :type "Key Structure"))
  (:`Pressed`
    (`KismetSystemLibrary.ExecuteConsoleCommand` "stat unit" null)))

(event `Key|F3`
  (params (Key :type "Key Structure"))
  (:`Pressed`
    (`/Engine/EditorBlueprintResources/StandardMacros.FlipFlop`
      (:`A`
        (`KismetSystemLibrary.ExecuteConsoleCommand` "viewmode unlit" null))
      (:`B`
        (`KismetSystemLibrary.ExecuteConsoleCommand` "viewmode lit" null)))))

(event `Key|F4`
  (params (Key :type "Key Structure"))
  (:`Pressed`
    (`/Engine/EditorBlueprintResources/StandardMacros.FlipFlop`
      (:`A`
        (`KismetSystemLibrary.ExecuteConsoleCommand` "r.Screenpercentage 50" null))
      (:`B`
        (`KismetSystemLibrary.ExecuteConsoleCommand` "r.Screenpercentage 100" null)))))

(event `Key|F5`
  (params (Key :type "Key Structure"))
  (:`Pressed`
    (`/Engine/EditorBlueprintResources/StandardMacros.FlipFlop`
      (:`A`
        (`KismetSystemLibrary.ExecuteConsoleCommand` "r.SetRes 1280x720" null))
      (:`B`
        (`KismetSystemLibrary.ExecuteConsoleCommand` "r.SetRes 1280x720w" null)))))

(event `Key|F6`
  (params (Key :type "Key Structure"))
  (:`Pressed`
    (`/Engine/EditorBlueprintResources/StandardMacros.FlipFlop`
      (:`A`
        (`KismetSystemLibrary.ExecuteConsoleCommand` "r.SetRes 1920x1080" null))
      (:`B`
        (`KismetSystemLibrary.ExecuteConsoleCommand` "r.SetRes 1920x1080w" null)))))

(fn `EndDialog`
  (set `self.inDialog` false)
  (`self.EnableInput` (`self.K2_GetPawn`) null)
  (`self.DialogEnded`))

(fn `StartDialog`
  (params (Dialog :type "/Game/BP/Struct/Dialog_Struct Structure"))
  (set `self.inDialog` true)
  (bind _returnvalue (`|CreateWidget` "/Game/UI/UI_Dialog.UI_Dialog_C" null Dialog))
  (bind _output_get (set `self.DialogWidgetRef` _returnvalue))
  (`UserWidget.AddToViewport` _output_get 0)
  (`self.DisableInput` (`self.K2_GetPawn`) null))

(fn `UserConstructionScript`)