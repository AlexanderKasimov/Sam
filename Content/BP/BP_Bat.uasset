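; BP_Bat is a bat actor that bobs back and forth along its up axis around its spawn location.
; On BeginPlay it stores that location and direction, then starts moving after a short random delay.
; Each Tick it flips direction whenever it is beyond a fixed distance from the origin, then applies a swept, frame-rate-scaled move at MovementSpeed.
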(event `self.ReceiveBeginPlay`
  (set `self.DefaultLocation` (`self.K2_GetActorLocation`))
  (set `self.MovementDirection` (`self.GetActorUpVector`))
  (`KismetSystemLibrary.K2_SetTimerDelegate` (delegate `StartMoving`) (`KismetMathLibrary.RandomFloatInRange` 0.0 3.0)))

(event `StartMoving`
  (set `self.isMoving` true))

(event `self.ReceiveActorBeginOverlap`
  (params (OtherActor :type "Actor Object Reference")))

(event `self.ReceiveTick`
  (params (DeltaSeconds :type "Float (single-precision)"))
  (if (`self.isMoving`)
    (`|ExecutionSequence`
      (:`then_0`
        (if (> (`KismetMathLibrary.VSize` (- (`self.DefaultLocation`) (`self.K2_GetActorLocation`))) 20.0)
          (set `self.MovementDirection` (* (`self.MovementDirection`) -1.0))))
      (:`then_1`
        (`self.K2_SetActorLocation` (+ (`self.K2_GetActorLocation`) (* (`self.MovementDirection`) (* (`self.MovementSpeed`) (`GameplayStatics.GetWorldDeltaSeconds`)))) true)))))

(fn `UserConstructionScript`
  (`parent.UserConstructionScript`))